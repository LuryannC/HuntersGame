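; BP_WorldManager tracks the player's real-world GPS state, seeding player coordinates from test longitude and latitude.
; PlayerInitiated binds to the controller's GeoHeading and GeoLocation delegates, and location updates store bearing and speed.
; Android also binds location-service changes, but that handler and the heading handler are empty.
; BP_GetGPSVelocity, uncalled here, derives speed from distance over timestamp delta between successive last-known locations.
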(event `self.ReceiveBeginPlay`
  (set `self.PlayerCoords` (make `PlayerCoords` (`self.TestLongitude`) (`self.TestLatitude`)))
  (if (`KismetStringLibrary.Contains` (`GameplayStatics.GetPlatformName`) "Android")
    (bind _returnvalue (`LocationServices.GetLocationServicesImpl`))
    (add `LocationServicesImpl.OnLocationChanged` _returnvalue (`|CreateDelegate` :!event `OnLocationChanged`))))

(event `OnLocationChanged`
  (params (LocationData :type "LocationServicesData Structure")))

(event `PlayerInitiated`
  (params (PlayerController :type "/Game/TopDown/Blueprints/BP_TopDownPlayerController Object Reference"))
  (add `GeoHeadingComponent.HeadingUpdateDelegate` (`/Game/TopDown/Blueprints/BP_TopDownPlayerController.GeoHeading` PlayerController) (`|CreateDelegate` :!event `OnGeoHeadingUpdated`))
  (add `GeoLocationComponent.LocationUpdateDelegate` (`HuntersGamePlayerController.GeoLocation` PlayerController) (`|CreateDelegate` :!event `OnGeoLocationUpdated`)))

(event `OnGeoHeadingUpdated`
  (params (heading :type "GeoHeading Structure")))

(event `OnGeoLocationUpdated`
  (params (position :type "GeoLocationPosition Object Reference"))
  (bind _returnvalue (`GeoLocationPosition.GetBearing` position))
  (set `self.Bearing` _returnvalue)
  (bind _returnvalue_2 (`GeoLocationPosition.GetSpeed` position))
  (set `self.Speed` _returnvalue_2))

(fn `BP_GetGPSVelocity`
  (returns (Speed :type "Float (double-precision)"))
  (locals (CurrentLocation :type "LocationServicesData Structure") (Distance :type "Float (double-precision)") (TimeDelta :type "Float (double-precision)") (CurrentSpeed :type "Float (double-precision)"))
  (bind _bppreviouslocatio_timestamp (break `LocationServicesData` (`self.BPPreviousLocatio`)))
  (bind _currentlocation_timestamp (break `LocationServicesData` (`local.CurrentLocation`)))
  (bind (_bppreviouslocatio_timestamp_2 _bppreviouslocatio_longitude _bppreviouslocatio_latitude) (break `LocationServicesData` (`self.BPPreviousLocatio`)))
  (bind (_currentlocation_timestamp_2 _currentlocation_longitude _currentlocation_latitude) (break `LocationServicesData` (`local.CurrentLocation`)))
  (bind _returnvalue (`LocationServices.AreLocationServicesEnabled`))
  (if _returnvalue
    (bind _returnvalue_2 (`LocationServices.GetLastKnownLocation`))
    (set `local.CurrentLocation` _returnvalue_2)
    (if (`self.bHasLocation`)
      (bind _returnvalue_3 (`self.CalculateDistance` _bppreviouslocatio_latitude _bppreviouslocatio_longitude _currentlocation_latitude _currentlocation_longitude))
      (set `local.Distance` _returnvalue_3)
      (set `local.TimeDelta` (/ (- _currentlocation_timestamp _bppreviouslocatio_timestamp) 1000.0))
      (if (> (`local.TimeDelta`) 0.0)
        (set `local.CurrentSpeed` (/ (`local.Distance`) (`local.TimeDelta`)))
        (set `self.BPPreviousLocatio` (`local.CurrentLocation`))
        (return (`local.CurrentSpeed`)))
      (else
        (set `self.BPPreviousLocatio` (`local.CurrentLocation`))
        (set `self.bHasLocation` true)
        (return 0.0)))
    (else
      (`KismetSystemLibrary.PrintString` "Location Services Disabled")
      (return 0.0))))

(fn `UserConstructionScript`)